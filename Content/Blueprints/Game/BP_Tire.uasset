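; BP_Tire is a physics-driven rolling tire that acts as the player character and becomes a "king" mesh on touching the victory box.
; Tick applies torque along the current direction and runs two downward traces to enable impulse jumps.
; Direction changes brake the roll with temporary angular damping, which suspends torque until a timer resets it.
; It also handles pausing via time dilation, level restart, and saving transform-related state on keypress or EndPlay.
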(event `self.ReceiveBeginPlay`
  (`self.BecomeKing`))

(event `self.ReceiveTick`
  (params (DeltaSeconds :type "Float (single-precision)"))
  (bind _returnvalue (- (`self.K2_GetActorLocation`) (`KismetMathLibrary.MakeVector` -75.0 0.0 (`self.LineOffset`))))
  (bind _returnvalue_2 (- (`self.K2_GetActorLocation`) (`KismetMathLibrary.MakeVector` 75.0 0.0 (`self.LineOffset`))))
  (if (`self.CanExecute`)
    (`self.MoveRight` (`self.CurrentDirection`))
    (bind (_outhit _returnvalue_3) (`KismetSystemLibrary.LineTraceSingle` _returnvalue (+ _returnvalue (* (`KismetMathLibrary.Vector_Down`) 35.0)) "TraceTypeQuery1"))
    (if _returnvalue_3
      (set `self.CanJump` _returnvalue_3)
      (else
        (bind (_outhit_2 _returnvalue_4) (`KismetSystemLibrary.LineTraceSingle` _returnvalue_2 (+ _returnvalue_2 (* (`KismetMathLibrary.Vector_Down`) 50.0)) "TraceTypeQuery1"))
        (set `self.CanJump` _returnvalue_4)))))

(event `Key|R`
  (params (Key :type "Key Structure"))
  (:`Pressed`
    (`GameplayStatics.OpenLevel` "MainMap")))

(event `Key|P`
  (params (Key :type "Key Structure"))
  (:`Pressed`
    (`GameplayStatics.SetGlobalTimeDilation` 0.0)))

(event `self.TireCol.OnComponentBeginOverlap`
  (params (OverlappedComponent :type "PrimitiveComponent Object Reference") (OtherActor :type "Actor Object Reference") (OtherComp :type "PrimitiveComponent Object Reference") (OtherBodyIndex :type Integer) (bFromSweep :type Boolean) (SweepResult :type "HitResult Structure (by ref)"))
  (if (== (`GameplayStatics.GetObjectClass` OtherActor) "/Game/Blueprints/Game/BP_VictoryBox.BP_VictoryBox_C")
    (set `self.IsKing` true)
    (`self.BecomeKing`)))

(event `Key|L`
  (params (Key :type "Key Structure"))
  (:`Pressed`
    (bind _success (`self.SaveGame`))
    (`KismetSystemLibrary.PrintString` "SAVED" _success)))

(event `self.ReceiveEndPlay`
  (params (EndPlayReason :type "EEndPlayReason Enum" :default "Destroyed"))
  (bind _success (`self.SaveGame`))
  (`KismetSystemLibrary.PrintString` "SAVED" _success))

(fn `BecomeKing`
  (if (`self.IsKing`)
    (`StaticMeshComponent.SetStaticMesh` (`self.Tire`) "/Game/Models/Tire/KingTire.KingTire")))

(fn `ChangeDirection`
  (params (Direction :type "Float (double-precision)"))
  (if (`self.CanExecute`)
    (set `self.currentDirection` Direction)
    (`PrimitiveComponent.SetAngularDamping` (`self.TireCol`) 13.0)
    (`KismetSystemLibrary.K2_SetTimer` self "ResetAngularSpeed" 0.4)))

(fn `Jump`
  (if (and (`self.CanJump`) (`self.CanExecute`))
    (`PrimitiveComponent.AddImpulse` (`self.TireCol`) (`KismetMathLibrary.MakeVector` 0.0 0.0 (`self.JumpImpulse`)) "None" false)
    (set `self.CanJump` false) ; Disallow jumping
  ))

(fn `MoveRight`
  (params (Direction :type "Float (double-precision)"))
  (bind _tirecol (`self.TireCol`))
  (if (== (`PrimitiveComponent.GetAngularDamping` _tirecol) 0.0)
    (`PrimitiveComponent.AddTorqueInRadians` _tirecol (`KismetMathLibrary.MakeVector` (* (`self.RollTorque`) Direction -1.0)) "None" false)))

(fn `PauseGame`
  (`GameplayStatics.SetGlobalTimeDilation` 0.0)
  (set `self.CanExecute` false))

(fn `ResetAngularSpeed`
  (`PrimitiveComponent.SetAngularDamping` (`self.TireCol`) 0.0))

(fn `SaveGame`
  (returns (Success :type Boolean))
  (bind _tirecol (`self.TireCol`))
  (bind _returnvalue (`GameplayStatics.CreateSaveGameObject` "/Game/Blueprints/Game/BP_PlayerInfo.BP_PlayerInfo_C"))
  (bind _returnvalue_2 (`PrimitiveComponent.GetPhysicsLinearVelocity` _tirecol "None"))
  (set `/Game/Blueprints/Game/BP_PlayerInfo.PlayerInfo` (make `/Game/Blueprints/Game/PlayerInfoStruct` (`self.K2_GetActorLocation`) (`self.CurrentDirection`) _returnvalue_2 (`PrimitiveComponent.GetPhysicsAngularVelocityInRadians` _tirecol "None") (`self.IsKing`)) _returnvalue)
  (bind _returnvalue_3 (`GameplayStatics.SaveGameToSlot` _returnvalue (`KismetSystemLibrary.GetPlatformUserName`)))
  (return _returnvalue_3))

(fn `UnPauseGame`
  (`GameplayStatics.SetGlobalTimeDilation` 1.0)
  (set `self.CanExecute` true))

(fn `UserConstructionScript`)