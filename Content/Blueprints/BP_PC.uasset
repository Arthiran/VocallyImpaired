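; Player controller that lets the player steer and jump a BP_Tire pawn by voice.
; On BeginPlay it restores the tire's location, direction, velocities and win state from the save slot named after the platform user, if one exists.
; It then spawns and tunes a SpeechRecognitionActor in keyword mode, mapping "jump", "left" and "right" to tire actions.
; EndPlay shuts recognition down.
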(event `self.ReceiveBeginPlay`
  (bind _returnvalue (`KismetSystemLibrary.GetPlatformUserName`))
  (`GameplayStatics.DoesSaveGameExist` _returnvalue)
  (if true
    (bind _returnvalue_2 (`GameplayStatics.LoadGameFromSlot` _returnvalue))
    (bind _asbp_player_info (cast `/Game/Blueprints/BP_PlayerInfo` _returnvalue_2))
    (bind _asbp_tire (cast `/Game/Blueprints/BP_Tire` (`GameplayStatics.GetPlayerPawn` 0)))
    (bind (_playerinfo_playerlocation _playerinfo_currentdirection _playerinfo_linearvelocity _playerinfo_angularvelocity _playerinfo_haswon) (break `/Game/Blueprints/PlayerInfo` (`/Game/Blueprints/BP_PlayerInfo.PlayerInfo` _asbp_player_info)))
    (`self.K2_SetActorLocation` _asbp_tire _playerinfo_playerlocation false false)
    (`/Game/Blueprints/BP_Tire.ChangeDirection` _asbp_tire _playerinfo_currentdirection)
    (bind _tirecol (`/Game/Blueprints/BP_Tire.TireCol` _asbp_tire))
    (`PrimitiveComponent.SetPhysicsLinearVelocity` _tirecol _playerinfo_linearvelocity false "None")
    (`PrimitiveComponent.SetPhysicsAngularVelocityInRadians` _tirecol _playerinfo_angularvelocity false "None")
    (bind _returnvalue_3 (`PrimitiveComponent.GetPhysicsLinearVelocity` (`/Game/Blueprints/BP_Tire.TireCol` _asbp_tire) "None"))
    (`KismetSystemLibrary.PrintString` (`KismetStringLibrary.Conv_VectorToString` _returnvalue_3))
    (set `/Game/Blueprints/BP_Tire.IsKing` _playerinfo_haswon _asbp_tire))
  ;[0 1 0.6469] Initialize Speech Recognition Plugin
  (bind _returnvalue_4 (`|SpawnActorFromClass` "/Script/SpeechRecognition.SpeechRecognitionActor" (`self.GetTransform`) "Undefined" "OverrideRootScale" null null))
  (bind _output_get (set `self.SpeechRecognitionPtr` _returnvalue_4))
  (add `SpeechRecognitionActor.OnStartedSpeaking` _output_get (delegate `StartedSpeakingEvent`))
  (add `SpeechRecognitionActor.OnWordsSpoken` _output_get (delegate `EventWordsSpoken`))
  (bind _returnvalue_5 (`SpeechRecognitionActor.Init` (`self.SpeechRecognitionPtr`) "VE_English"))
  (if _returnvalue_5
    (`self.SetConfig`)
    (`SpeechRecognitionActor.EnableKeywordMode` (`self.SpeechRecognitionPtr`) (`|MakeArray` (make `RecognitionPhrase` "jump" 15) (make `RecognitionPhrase` "right" 15) (make `RecognitionPhrase` "left" 15)))
    (`KismetSystemLibrary.Delay` 0.2)
    (bind _asbp_tire_2 (cast `/Game/Blueprints/BP_Tire` (`GameplayStatics.GetPlayerPawn` 0)))
    (set `self.CharacterVar` _asbp_tire_2)
    (else
      (`KismetSystemLibrary.PrintString` "Speech Rec Failed"))))

(event `EventWordsSpoken`
  (params (Text :type "RecognisedPhrases Structure"))
  ;[0 1 0.6469] Initialize Speech Recognition Plugin
  (`self.WordsSpoken` Text))

(event `StartedSpeakingEvent`
  ;[0 1 0.6469] Initialize Speech Recognition Plugin
  (`self.StartedSpeaking`))

(event `self.ReceiveEndPlay`
  (params (EndPlayReason :type "EEndPlayReason Enum" :default "Destroyed"))
  ;[0 1 0.6469] Initialize Speech Recognition Plugin
  (`SpeechRecognitionActor.Shutdown` (`self.SpeechRecognitionPtr`)))

(fn `SetConfig`
  (`self.SetConfigParam` "-vad_prespeech" "VE_INTEGER" "30")
  (`self.SetConfigParam` "-vad_postspeech" "VE_INTEGER" "30"))

(fn `SetConfigParam`
  (params (Param :type String) (Type :type "ESpeechRecognitionParamType Enum" :default "VE_FLOAT") (Value :type String))
  (`SpeechRecognitionActor.SetConfigParam` (`self.SpeechRecognitionPtr`) Param Type Value))

(fn `StartedSpeaking`)

(fn `UserConstructionScript`)

(fn `WordsSpoken`
  (params (NewParam :type "RecognisedPhrases Structure"))
  (bind _charactervar (`self.CharacterVar`))
  (switch `string` (`.phrase` (break `DetectedPhrase` (`|GetArrayItem` (`.phrases` (break `RecognisedPhrases` NewParam)))))
    (:`jump`
      (`/Game/Blueprints/BP_Tire.Jump` _charactervar))
    (:`right`
      (`/Game/Blueprints/BP_Tire.ChangeDirection` _charactervar -1.0))
    (:`left`
      (`/Game/Blueprints/BP_Tire.ChangeDirection` _charactervar 1.0))))