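; BP_Tire is a physics-driven rolling tire actor that moves along one axis and can jump.
; Each tick it applies roll torque from CurrentDirection to TireCol and runs a short downward line trace to set CanJump.
; ChangeDirection sets a new direction and briefly raises angular damping, cleared by a timer, to brake the spin.
; Jump applies an upward impulse when CanJump is true.
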(event `self.ReceiveTick`
  (params (DeltaSeconds :type "Float (single-precision)"))
  (bind _returnvalue (- (`self.K2_GetActorLocation`) (`KismetMathLibrary.MakeVector` 0.0 0.0 (`self.LineOffset`))))
  (`self.MoveRight` (`self.CurrentDirection`))
  (bind (_outhit _returnvalue_2) (`KismetSystemLibrary.LineTraceSingle` _returnvalue (+ _returnvalue (* (`KismetMathLibrary.Vector_Down`) 28.0)) "TraceTypeQuery1"))
  (set `self.CanJump` _returnvalue_2))

(fn `ChangeDirection`
  (params (Direction :type "Float (double-precision)"))
  (set `self.currentDirection` Direction)
  (`PrimitiveComponent.SetAngularDamping` (`self.TireCol`) 15.0)
  (`KismetSystemLibrary.K2_SetTimer` self "ResetAngularSpeed" 0.5))

(fn `Jump`
  (if (`self.CanJump`)
    (`KismetSystemLibrary.PrintString` "WE JUMPIN")
    (`PrimitiveComponent.AddImpulse` (`self.TireCol`) (`KismetMathLibrary.MakeVector` 0.0 0.0 (`self.JumpImpulse`)) "None" false)
    (set `self.CanJump` false) ; Disallow jumping
  ))

(fn `MoveRight`
  (params (Direction :type "Float (double-precision)"))
  (`PrimitiveComponent.AddTorqueInRadians` (`self.TireCol`) (`KismetMathLibrary.MakeVector` 0.0 (* (`self.RollTorque`) Direction -1.0)) "None" false))

(fn `ResetAngularSpeed`
  (`PrimitiveComponent.SetAngularDamping` (`self.TireCol`) 0.0))

(fn `UserConstructionScript`)